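; VR pawn for the FileBrowser content that sets up the headset and lets the player interact with widgets.
; On BeginPlay it enables the HMD, sets floor tracking and resets orientation for Oculus and SteamVR devices, and sets VR pixel density by console command.
; R or either controller grip re-centers orientation.
; Either trigger drives the WidgetInteraction component as a left mouse press and release.
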(event `self.ReceiveBeginPlay`
  (`|ExecutionSequence`
    (:`then_0`
      ;[1 1 1] Setup Player Height for various Platforms (Vive, Oculus)
      (`HeadMountedDisplayFunctionLibrary.EnableHMD` true)
      (switch `name` (`HeadMountedDisplayFunctionLibrary.GetHMDDeviceName`)
        (:`OculusHMD`
          _)
        (:`SteamVR`
          _))
      (`HeadMountedDisplayFunctionLibrary.SetTrackingOrigin` "Floor") ; Windows (Oculus / Vive)
      (`HeadMountedDisplayFunctionLibrary.ResetOrientationAndPosition` 0.0 "Orientation"))
    (:`then_1`
      ;[1 1 1] PixelDensity
      (`KismetSystemLibrary.ExecuteConsoleCommand` "vr.PixelDensity 1.0" null))))

(event `Key|R`
  (params (Key :type "Key Structure"))
  ;[1 1 1] Reset Orientation and position
  (:`Pressed`
    (`HeadMountedDisplayFunctionLibrary.SetTrackingOrigin` "Floor" :!label _label) ; Windows (Oculus / Vive)
    (`HeadMountedDisplayFunctionLibrary.ResetOrientationAndPosition` 0.0 "Orientation")))

(event `Key|MotionController_Left_Grip1`
  (params (Key :type "Key Structure"))
  ;[1 1 1] Reset Orientation and position
  (:`Pressed`
    (goto _label)))

(event `Key|MotionController_Right_Grip1`
  (params (Key :type "Key Structure"))
  ;[1 1 1] Reset Orientation and position
  (:`Pressed`
    (goto _label)))

(event `Key|MotionController_Left_Trigger`
  (params (Key :type "Key Structure"))
  (bind _widgetinteraction (`self.WidgetInteraction`))
  ;[1 1 1] Iterraction
  (:`Pressed`
    (`WidgetInteractionComponent.PressPointerKey` _widgetinteraction "LeftMouseButton" :!label _label_2))
  (:`Released`
    (`WidgetInteractionComponent.ReleasePointerKey` _widgetinteraction "LeftMouseButton" :!label _label_3)))

(event `Key|MotionController_Right_Trigger`
  (params (Key :type "Key Structure"))
  ;[1 1 1] Iterraction
  (:`Pressed`
    (goto _label_2))
  (:`Released`
    (goto _label_3)))

(fn `UserConstructionScript`)